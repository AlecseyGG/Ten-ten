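; Player controller for touch drag-and-drop of a ControlActor in a grid-based block game, with the mouse cursor shown.
; Touch press rescales the actor and stores its position; movement follows the deprojected touch point at fixed height.
; Release fires the mesh and grid-check dispatchers, returns the actor to its start, then calls StateActor if no BP_BaseActor remains; Q also calls it.
; ChekActiveGrid is an empty stub with unconnected block-scanning logic.
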(event EventBeginPlay
  ;[1 1 1] Show mouse cursor
  (Variables|Default|SetbShowMouseCursor true))

(event Input|KeyboardEvents|Q
  (params (Key :type Key%20Structure :default "None"))
  (:Pressed
    (Default|CallEDStateActor)))

(event Input|TouchEvents|InputTouch
  (params (Location :type Vector) (FingerIndex :type ETouchIndex%20Enum))
  (bind _returnvalue (Game|GetPlayerController 0))
  (bind _controlactor (Variables|Default|GetControlActor))
  (bind _worldlocation (Class|PlayerController|DeprojectScreenPositiontoWorld _returnvalue (.x Location) (.y Location)))
  (:Pressed
    (Transformation|SetActorScale3D _controlactor "0.100000,0.100000,0.100000")
    (Variables|Default|SetStarterPosition (Transformation|GetActorLocation _controlactor)))
  (:Released
    (Default|CallEDActorMesh)
    (Default|CallEDCheckVoidGameGrid)
    (Transformation|SetActorLocation (Variables|Default|GetControlActor) (Variables|Default|GetStarterPosition) false false)
    (CallFunction|CheckActiveActor))
  (:Moved
    (Transformation|SetActorLocation (Variables|Default|GetControlActor) (Math|Vector|MakeVector (.x _worldlocation) (.y _worldlocation) 0.5) false false)))

(fn ConstructionScript)

(fn CheckActiveActor
  (bind _outactors (Actor|GetAllActorsOfClass "/Game/Blueprint/Actor/BP_BaseActor.BP_BaseActor_C"))
  (if (< (Utilities|Array|Length _outactors) 1)
    (Default|CallEDStateActor)))

(fn ChekActiveGrid)