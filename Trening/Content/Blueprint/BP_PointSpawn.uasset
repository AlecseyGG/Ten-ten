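; BP_PointSpawn spawns a row of three small, randomly chosen piece actors at fixed positions along the Y axis.
; It spawns a set on BeginPlay and another whenever BP_PlayerController's ED_StateActor dispatcher, bound at startup, fires.
; GetRandomActor rolls an E_PickActor value per piece, but its four cases resolve to only two classes: Box and Line give BP_LineActor, Corner and Dot give DotActor.
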(event Custom|ED_StateActor_Event_0
  (CallFunction|SpawnActor))

(event EventBeginPlay
  (CallFunction|SpawnActor)
  (bind _asbp_player_controller (Utilities|Casting|CastToBP_PlayerController (Game|GetPlayerController 0)))
  (EventDispatchers|AssignEDStateActor _asbp_player_controller (delegate Custom|ED_StateActor_Event_0)))

(fn ConstructionScript)

(fn GetRandomActor
  (bind _output_get (Variables|Default|SetPickActor (Utilities|Enum|ByteToEnumE_PickActor (Math|Conversions|ToByte(Integer) (Math|Random|RandomIntegerinRange 0 3)))))
  (switch Utilities|FlowControl|Switch|SwitchonE_PickActor _output_get
    (:NewEnumerator0
      (return "/Game/Blueprint/Actor/BP_LineActor.BP_LineActor_C"))
    (:NewEnumerator3
      (return "/Game/Blueprint/Actor/DotActor.DotActor_C"))
    (:NewEnumerator1
      (return "/Game/Blueprint/Actor/DotActor.DotActor_C"))
    (:NewEnumerator2
      (return "/Game/Blueprint/Actor/BP_LineActor.BP_LineActor_C"))))

(fn SpawnActor
  (for _index (range 1 3)
    (Game|SpawnActorfromClass (CallFunction|GetRandomActor) (Math|Transform|MakeTransform (Math|Vector|MakeVector 0.0 (* _index -2e+01) 2.0) "0, 0, 0" "0.060000,0.060000,0.060000") "Undefined" 0 0)))