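; BP_CornerActor is a composite figure actor that assembles itself at BeginPlay from four BP_ActorMesh actors.
; It spawns each mesh at a small uniform scale, using the CornerPosition entries in ActorPosition, and records it in the EltmentFiguraIsActor array.
; Each mesh attaches to the actor with relative location and rotation and world scale, so the stored positions act as local offsets.
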(event EventBeginPlay
  (for _index (range 0 3)
    (bind _returnvalue (Game|SpawnActorfromClass "/Game/Blueprint/Actor/BP_ActorMesh.BP_ActorMesh_C" (Math|Transform|MakeTransform (Utilities|Array|Get(acopy) (.CornerPosition (Utilities|Struct|BreakActorPosition (Variables|Default|GetActorPosition))) _index) "0, 0, 0" "0.060000,0.060000,0.060000") "Undefined" 0 0))
    (Utilities|Array|Add (Variables|Default|GetEltmentFiguraIsActor) _returnvalue)
    (Transformation|AttachActorToActor _returnvalue self "None" "KeepRelative" "KeepRelative" "KeepWorld" true)))

(fn ConstructionScript
  (|CallParentFunction))