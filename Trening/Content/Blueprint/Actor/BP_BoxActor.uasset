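; BP_BoxActor is an actor that builds a group of small BP_ActorMesh pieces on itself at BeginPlay.
; A nested loop spawns each piece at reduced scale, stores it in EltmentFiguraIsActor and attaches it to the box, keeping relative location and rotation and world scale.
; Spawn locations come from ActorPosition.BoxPosition, indexed by the product of the two loop counters, so several pieces share positions.
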(event EventBeginPlay
  (|CallParentFunction)
  (for _index (range 0 2)
    (for _index_2 (range 0 2)
      (bind _returnvalue (Game|SpawnActorfromClass "/Game/Blueprint/Actor/BP_ActorMesh.BP_ActorMesh_C" (Math|Transform|MakeTransform (Utilities|Array|Get(acopy) (.BoxPosition (Utilities|Struct|BreakActorPosition (Variables|Default|GetActorPosition))) (* _index_2 _index)) "0, 0, 0" "0.060000,0.060000,0.060000") "Undefined" 0 0))
      (Utilities|Array|Add (Variables|Default|GetEltmentFiguraIsActor) _returnvalue)
      (Transformation|AttachActorToActor _returnvalue self "None" "KeepRelative" "KeepRelative" "KeepWorld" true))))

(fn ConstructionScript
  (|CallParentFunction))