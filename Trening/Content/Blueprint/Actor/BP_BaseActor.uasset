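; BP_BaseActor is a touch-controlled figure made of element actors that gets placed onto BP_BaseBlock grid blocks.
; Touch begin registers it as the player controller's ControlActor; touch end binds placement to the controller's EDActorMesh dispatcher.
; Placement collects each element's trace-hit block, stopping at the first with a false state.
; If all pass, it attaches elements to trace results, sets block states true and destroys itself.
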(event Custom|CustomEvent_0
  ;[1 1 1] Comment
  (CallFunction|GetComponentControlActor))

(event EventActorOnInputTouchBegin
  (params (FingerIndex :type ETouchIndex%20Enum :default "Touch1"))
  (Variables|/Game/Blueprint/BP_PlayerController.BP_PlayerController_C|SetControlActor (.AsBP%20Player%20Controller (Utilities|Casting|CastToBP_PlayerController (Game|GetPlayerController 0))) self))

(event EventActorOnInputTouchEnd
  (params (FingerIndex :type ETouchIndex%20Enum :default "Touch1"))
  ;[1 1 1] Comment
  (bind _asbp_player_controller (Utilities|Casting|CastToBP_PlayerController (Game|GetPlayerController 0)))
  (EventDispatchers|AssignEDActorMesh _asbp_player_controller (delegate Custom|CustomEvent_0)))

(fn ConstructionScript)

(fn GetComponentControlActor
  (bind _eltmentfiguraisactor (Variables|Default|GetEltmentFiguraIsActor))
  (bind _array_element (Utilities|Array|ForEachLoopwithBreak _eltmentfiguraisactor :!label _label)
    (:LoopBody
      (bind _hitactor (Default|GetResultTrase _array_element))
      (bind _asbp_base_block (Utilities|Casting|CastToBP_BaseBlock _hitactor))
      (bind _isactive (Default|GetterStateBlock _asbp_base_block))
      (if _isactive
        (Utilities|Array|Add (Variables|Default|GetGet%20ActorGrid) _hitactor)
        (else
          (goto _label Break))))
    (:Completed
      (if (== (Utilities|Array|Length _eltmentfiguraisactor) (Utilities|Array|Length (Variables|Default|GetGet%20ActorGrid)))
        (for (_array_element_2 _array_index) (Variables|Default|GetEltmentFiguraIsActor)
          (Transformation|AttachActorToActor _array_element_2 _hitactor "None" "KeepRelative" "KeepRelative" "KeepRelative" true)
          (bind _asbp_base_block_2 (Utilities|Casting|CastToBP_BaseBlock (Utilities|Array|Get(acopy) (Variables|Default|GetGet%20ActorGrid) _array_index)))
          (Default|SetterStateBlock _asbp_base_block_2 true))
        (Actor|DestroyActor self)))))