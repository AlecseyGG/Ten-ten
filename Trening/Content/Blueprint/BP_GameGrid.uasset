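; BP_GameGrid builds the board for a block puzzle and clears its full rows and columns.
; On BeginPlay it spawns BP_BaseBlock cells into a nested 2D array and registers a check event with BP_PlayerController.
; When that event fires, CheckStateGrid counts cell states along each row and column.
; DestroyCoponent clears a full line by destroying the actors attached to its cells.
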(event Custom|ED_CheckVoidGameGrid_Event_0
  (CallFunction|CheckStateGrid))

(event EventBeginPlay
  (CallFunction|CreateGameGrid)
  (bind _asbp_player_controller (Utilities|Casting|CastToBP_PlayerController (Game|GetPlayerController 0)))
  (EventDispatchers|AssignEDCheckVoidGameGrid _asbp_player_controller (delegate Custom|ED_CheckVoidGameGrid_Event_0)))

(fn ConstructionScript)

(fn CreateGameGrid
  (for _index (range 0 (Variables|Default|GetsizeY))
    (Variables|Default|SetArrayX "")
    (for _index_2 (range 0 (Variables|Default|GetsizeX))
      (bind _returnvalue (Game|SpawnActorfromClass "/Game/Blueprint/Actor/BP_BaseBlock.BP_BaseBlock_C" (Math|Transform|MakeTransform (Math|Vector|MakeVector (* _index_2 11.0) (* _index 11.0) 0.1) "0, 0, 0" "0.100000,0.100000,0.100000") "Undefined" 0 0))
      (Utilities|Array|Add (Utilities|Struct|BreakBP_StractArrayGameGrid (Variables|Default|GetArrayX)) _returnvalue))
    (Utilities|Array|Add (Variables|Default|GetArrayY) (Variables|Default|GetArrayX))))

(fn DestroyCoponent
  (params (Horisontal :type Integer) (Vertical :type Integer))
  (if (> Horisontal 0)
    ;[1 1 1] Уничтожение по вертикали
    (for _index (range Horisontal Horisontal)
      (for _index_2 (range 0 (Variables|Default|GetsizeX))
        (Actor|DestroyActor (Actor|GetAttachedActors (Utilities|Array|Get(acopy) (Utilities|Struct|BreakBP_StractArrayGameGrid (Utilities|Array|Get(acopy) (Variables|Default|GetArrayY) _index)) _index_2) true))))
    (else
      ;[1 1 1] Уничтожение по горизонтали
      (for _index_3 (range Vertical Vertical)
        (for _index_4 (range 0 (Variables|Default|GetsizeY))
          (Actor|DestroyActor (Actor|GetAttachedActors (Utilities|Array|Get(acopy) (Utilities|Struct|BreakBP_StractArrayGameGrid (Utilities|Array|Get(acopy) (Variables|Default|GetArrayY) _index_4)) _index_3) true)))))))

(fn CheckStateGrid
  ;[1 1 1] Проверка по горизонтали
  (for _index (range 0 (Variables|Default|GetsizeY))
    (LocalVariables|SetCounter 0)
    (bind _index_2 (Utilities|FlowControl|ForLoopwithBreak 0 (Variables|Default|GetsizeX))
      (:LoopBody
        (bind _isactive (Default|GetterStateBlock (Utilities|Array|Get(acopy) (Utilities|Struct|BreakBP_StractArrayGameGrid (Utilities|Array|Get(acopy) (Variables|Default|GetArrayY) _index)) _index_2)))
        (if _isactive
          (Math|Integer|IncrementInt (LocalVariables|GetCounter))))
      (:Completed
        (if (> (LocalVariables|GetCounter) (Variables|Default|GetsizeX))
          (CallFunction|DestroyCoponent _index)))))
  ;[1 1 1] Проверка по ветикали
  (for _index_3 (range 0 (Variables|Default|GetsizeX))
    (LocalVariables|SetCounter 0)
    (bind _index_4 (Utilities|FlowControl|ForLoopwithBreak 0 (Variables|Default|GetsizeY))
      (:LoopBody
        (bind _isactive_2 (Default|GetterStateBlock (Utilities|Array|Get(acopy) (Utilities|Struct|BreakBP_StractArrayGameGrid (Utilities|Array|Get(acopy) (Variables|Default|GetArrayY) _index_4)) _index_3)))
        (if _isactive_2
          (Math|Integer|IncrementInt (LocalVariables|GetCounter))))
      (:Completed
        (if (> (LocalVariables|GetCounter) (Variables|Default|GetsizeX))
          (CallFunction|DestroyCoponent 0 _index_3))))))